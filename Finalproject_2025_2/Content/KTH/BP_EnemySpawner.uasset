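; Spawner actor that scatters walls and gems around itself at BeginPlay and keeps spawning enemies during play.
; Walls and gems use random navmesh-projected points within MapRadius, with square-root radius scaling for even spread and weighted random selection of wall classes.
; A looping timer adds one enemy while below MaxEnemyCount, placed on the navmesh in the half-ring behind the player between MinDistance and MaxDistance.
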(event Custom|SpawnEnemy
  (bind _enemyclass (Variables|Default|GetEnemyClass))
  (bind _outactors (Actor|GetAllActorsOfClass _enemyclass))
  (if (< (Utilities|Array|Length _outactors) (Variables|Default|GetMaxEnemyCount))
    (for _index (range 1 1)
      (bind _spawnlocation (CallFunction|GetValidSpawnLocation))
      (Game|SpawnActorfromClass _enemyclass (Math|Conversions|ToTransform(Vector) _spawnlocation) "Undefined" "MultiplyWithRoot" 0 0))))

(event Custom|CountBot
  ;[0.15 0.15 0.15 0.5] 나중에 삭제해도 됨. EnemyCount
)

(event Custom|SpawnGem
  (bind _returnvalue (Transformation|GetActorLocation))
  (bind _returnvalue_2 (Math|Random|RandomUnitVector))
  (bind _returnvalue_3 (Math|Random|RandomFloatinRange 0.0 1.0))
  (bind _mapradius (Variables|Default|GetMapRadius))
  (bind (_x _y) (Math|Vector|BreakVector _returnvalue_2))
  (bind _returnvalue_4 (Math|Float|Power _returnvalue_3 0.5))
  (bind _returnvalue_5 (Math|Vector|MakeVector _x _y 0.0))
  (bind _returnvalue_6 (* _returnvalue_4 _mapradius))
  (bind _returnvalue_7 (Math|Vector|Normalize _returnvalue_5))
  (bind _returnvalue_8 (* _returnvalue_7 _returnvalue_6))
  (bind _returnvalue_9 (+ _returnvalue _returnvalue_8))
  (bind (_projectedlocation _returnvalue_10) (AI|Navigation|ProjectPointtoNavigation _returnvalue_9 0 0 "0, 0, 0"))
  (for _index (range 1 (Variables|Default|GetTotalGemCount))
    (if _returnvalue_10
      (Game|SpawnActorfromClass (Variables|Default|GetGemClass) (Math|Transform|MakeTransform _projectedlocation (Math|Rotator|MakeRotator 0.0 0.0 (Math|Random|RandomFloatinRange 0.0 3.6e+02)) "1.000000,1.000000,1.000000") "AdjustIfPossibleButAlwaysSpawn" "MultiplyWithRoot" 0 0))))

(event Custom|SpawnWall
  (bind _returnvalue (Math|Random|RandomUnitVector))
  (bind _returnvalue_2 (Math|Random|RandomFloatinRange 0.0 1.0))
  (bind _returnvalue_3 (Transformation|GetActorLocation))
  (bind _mapradius (Variables|Default|GetMapRadius))
  (bind (_x _y) (Math|Vector|BreakVector _returnvalue))
  (bind _returnvalue_4 (Math|Float|Power _returnvalue_2 0.5))
  (bind _returnvalue_5 (Math|Vector|MakeVector _x _y 0.0))
  (bind _returnvalue_6 (* _returnvalue_4 _mapradius))
  (bind _returnvalue_7 (Math|Vector|Normalize _returnvalue_5))
  (bind _returnvalue_8 (* _returnvalue_7 _returnvalue_6))
  (bind _returnvalue_9 (+ _returnvalue_3 _returnvalue_8))
  (bind (_projectedlocation _returnvalue_10) (AI|Navigation|ProjectPointtoNavigation _returnvalue_9 0 0 "0, 0, 0"))
  (for _index (range 1 (Variables|Default|GetTotalWallCount))
    (if _returnvalue_10
      (bind _selectedclass (CallFunction|GetWeightedClass))
      (Game|SpawnActorfromClass _selectedclass (Math|Transform|MakeTransform _projectedlocation (Math|Rotator|MakeRotator 0.0 0.0 (Math|Random|RandomFloatinRange 0.0 3.6e+02)) "1.000000,1.000000,1.000000") "AdjustIfPossibleButAlwaysSpawn" "MultiplyWithRoot" 0 0))))

(event EventBeginPlay
  (CallFunction|SpawnWall)
  (CallFunction|SpawnGem)
  (Utilities|Time|SetTimerbyEvent (delegate Custom|SpawnEnemy) (Variables|Default|GetEnemySpawnRate) true)
  ;[0.15 0.15 0.15 0.5] 나중에 삭제해도 됨. EnemyCount
  (Utilities|Time|SetTimerbyEvent (delegate Custom|CountBot) 1.0 true))

(event EventTick
  (params (DeltaSeconds :type Float%20%28single-precision%29))
  ;[0.15 0.15 0.15 0.5] 나중에 삭제해도 됨. 적, 벽 스폰 위치 원
)

(fn ConstructionScript)

(fn GetValidSpawnLocation
  (bind _returnvalue (Game|GetPlayerCharacter 0))
  (bind _returnvalue_2 (Game|GetPlayerCharacter 0))
  (bind _returnvalue_3 (Math|Random|RandomFloatinRange -9e+01 9e+01))
  (bind _maxdistance (Variables|Default|GetMaxDistance))
  (bind _mindistance (Variables|Default|GetMinDistance))
  (bind _returnvalue_4 (Transformation|GetActorLocation _returnvalue_2))
  (bind _returnvalue_5 (Transformation|GetActorRotation _returnvalue))
  (bind _returnvalue_6 (Math|Random|RandomFloatinRange _mindistance _maxdistance))
  (bind _yaw (Math|Rotator|BreakRotator _returnvalue_5))
  (bind _returnvalue_7 (+ _yaw 1.8e+02))
  (bind _returnvalue_8 (+ _returnvalue_7 _returnvalue_3))
  (bind _returnvalue_9 (Math|Rotator|MakeRotator 0.0 0.0 _returnvalue_8))
  (bind _returnvalue_10 (Math|Vector|GetForwardVector _returnvalue_9))
  (bind _returnvalue_11 (* _returnvalue_10 _returnvalue_6))
  (bind _returnvalue_12 (+ _returnvalue_11 _returnvalue_4))
  (bind (_projectedlocation _returnvalue_13) (AI|Navigation|ProjectPointtoNavigation _returnvalue_12 0 0 "500.000000,500.000000,500.000000"))
  (Variables|Default|SetTempLocation _projectedlocation)
  (return (Variables|Default|GetTempLocation) _returnvalue_13))

(fn GetWeightedClass
  (Variables|Default|SetTotalSum 0.0)
  (for _array_element (Variables|Default|GetSpawnWeights)
    (Variables|Default|SetTotalSum (+ _array_element (Variables|Default|GetTotalSum))))
  (Variables|Default|SetRandomRoll (Math|Random|RandomFloatinRange 0.0 (Variables|Default|GetTotalSum)))
  (for (_array_element_2 _array_index) (Variables|Default|GetSpawnWeights)
    (if (<= (Variables|Default|GetRandomRoll) _array_element_2)
      (return (Utilities|Array|Get(acopy) (Variables|Default|GetSpawnClasses) _array_index))
      (else
        (Variables|Default|SetRandomRoll (- (Variables|Default|GetRandomRoll) _array_element_2))))))