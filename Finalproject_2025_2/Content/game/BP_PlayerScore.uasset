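; BP_PlayerScore runs the round's rules: countdown, score, break combo and jewelry goal.
; Object breaks score by multiplier and raise the combo, whose maintenance window shrinks linearly per level and drops one level on expiry.
; The tenth jewelry pickup opens a random BP_Goal as the player's escape point.
; Tick starts police audio in the final minute, shows the escape arrow once a target exists, and calls BP_UI's game end when time expires.
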(event Custom|GetobjectBreakSignal
  (bind _mcmtime (Variables|Default|GetMCMTime))
  (Variables|Default|Setbreakobject (+ (Variables|Default|Getbreakobject) 1.0))
  (Variables|Default|Setplayerscore (+ (Variables|Default|Getplayerscore) (* (Variables|Default|Getplayercombo) 1e+01)))
  (Variables|Default|SetComboMaintenanceTime (- _mcmtime (* (/ (- _mcmtime (Variables|Default|GetminCMTime)) 19.0) (- (Variables|Default|Getplayercombo) 1.0)))))

(event Custom|GetJewlry
  (Variables|Default|SetWinScore (+ (Variables|Default|GetWinScore) 1.0))
  (if (== (Variables|Default|GetWinScore) 1e+01)
    (bind _outactors (Actor|GetAllActorsOfClass "/Game/game/BP_Goal.BP_Goal_C"))
    (bind _asbp_first_person_character (Utilities|Casting|CastToBP_FirstPersonCharacter (Game|GetPlayerCharacter 0)))
    (bind _output_get (Variables|/Game/FirstPerson/Blueprints/BP_FirstPersonCharacter.BP_FirstPersonCharacter_C|SetTargetEscapePoint _asbp_first_person_character (Utilities|Array|Get(acopy) _outactors (Math|Random|RandomIntegerinRange 0 (Utilities|Array|LastIndex _outactors)))))
    (bind _asbp_goal (Utilities|Casting|CastToBP_Goal _output_get))
    (Default|GoalOpen _asbp_goal)))

(event EventBeginPlay
  (Variables|Default|SetGameTime 3e+02)
  (Variables|Default|Setplayerscore 0.0)
  (Variables|Default|Setbreakobject 0.0)
  (Variables|Default|SetComboMaintenanceTime 0.0)
  (Variables|Default|Setplayercombo 1.0)
  (Variables|Default|SetWinScore 0.0))

(event EventTick
  (params (DeltaSeconds :type Float%20%28single-precision%29))
  (bind _mcmtime (Variables|Default|GetMCMTime))
  (Utilities|FlowControl|Sequence
    (:then_0
      (Variables|Default|SetGameTime (- (Variables|Default|GetGameTime) DeltaSeconds))
      (Utilities|FlowControl|Sequence
        (:then_0
          (bind _asbp_first_person_character (Utilities|Casting|CastToBP_FirstPersonCharacter (Game|GetPlayerCharacter 0)))
          (if (Utilities|IsValid (Variables|/Game/FirstPerson/Blueprints/BP_FirstPersonCharacter.BP_FirstPersonCharacter_C|GetTargetEscapePoint _asbp_first_person_character))
            (if (<= (Variables|Default|GetGameTime) 6e+01)
              (Utilities|FlowControl|DoOnce false
                (:Completed
                  (bind _foundwidgets (Widget|GetAllWidgetsOfClass "/Game/game/BP_UI.BP_UI_C" true))
                  (Default|Showarrow (Utilities|Array|Get(acopy) _foundwidgets)))))))
        (:then_1
          (if (< (Variables|Default|GetGameTime) 0.0)
            (bind _foundwidgets_2 (Widget|GetAllWidgetsOfClass "/Game/game/BP_UI.BP_UI_C" true))
            (Default|Gameend (Utilities|Array|Get(acopy) _foundwidgets_2))))
        (:then_2
          (if (<= (Variables|Default|GetGameTime) 6e+01)
            (Utilities|FlowControl|DoOnce false
              (:Completed
                (bind _returnvalue (Audio|SpawnSound2D "/Game/sound/police_Cue.police_Cue" 1.0 1.0 0.0 0))
                (Variables|Default|SetPoliceBGM _returnvalue)))))))
    (:then_1
      (if (> (Variables|Default|GetComboMaintenanceTime) 0.0)
        (Variables|Default|SetComboMaintenanceTime (- (Variables|Default|GetComboMaintenanceTime) DeltaSeconds))
        (elif (> (Variables|Default|Getplayercombo) 1.0)
          (Variables|Default|Setplayercombo (- (Variables|Default|Getplayercombo) 1.0))
          (Variables|Default|Setbreakobject 0.0)
          (Variables|Default|SetComboMaintenanceTime (- _mcmtime (* (/ (- _mcmtime (Variables|Default|GetminCMTime)) 19.0) (- (Variables|Default|Getplayercombo) 1.0))))))
      (if (>= (Variables|Default|Getbreakobject) 1.0)
        (Variables|Default|Setbreakobject 0.0)
        (if (< (Variables|Default|Getplayercombo) (Variables|Default|Getmaxcombo))
          (Variables|Default|Setplayercombo (+ (Variables|Default|Getplayercombo) 1.0)))))))

(fn ConstructionScript)

(fn GetComboMainProgerss
  (bind _mcmtime (Variables|Default|GetMCMTime))
  (return (/ (Variables|Default|GetComboMaintenanceTime) (- _mcmtime (* (/ (- _mcmtime (Variables|Default|GetminCMTime)) 19.0) (- (Variables|Default|Getplayercombo) 1.0))))))