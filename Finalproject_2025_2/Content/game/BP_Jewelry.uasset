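; BP_Jewelry is a collectible jewelry pickup that rewards the first-person character with score.
; Overlapping its capsule gets the character's BPPlayerScore, calls GetJewlry on it, adds a fixed amount to Playerscore and destroys the pickup.
; Tick bobs the actor vertically on a game-time sine wave around its BeginPlay location and spins its Rotation component in yaw, scaled by delta time.
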(event OnComponentBeginOverlap(Capsule)
  (params (OverlappedComponent :type Primitive%20Component%20Object%20Reference) (OtherActor :type Actor%20Object%20Reference) (OtherComp :type Primitive%20Component%20Object%20Reference) (OtherBodyIndex :type Integer) (bFromSweep :type Boolean) (SweepResult :type Hit%20Result%20Structure%20%28by%20ref%29))
  (bind _asbp_first_person_character (Utilities|Casting|CastToBP_FirstPersonCharacter OtherActor))
  (bind _asbp_player_score (Default|GetBPPlayerScore _asbp_first_person_character))
  (Default|GetJewlry _asbp_player_score)
  (Variables|/Game/game/BP_PlayerScore.BP_PlayerScore_C|Setplayerscore _asbp_player_score (+ (Variables|/Game/game/BP_PlayerScore.BP_PlayerScore_C|Getplayerscore _asbp_player_score) 1e+02))
  (Actor|DestroyActor))

(event EventBeginPlay
  (Variables|Default|SetStartlocation (Transformation|GetActorLocation)))

(event Collision|EventActorBeginOverlap
  (params (OtherActor :type Actor%20Object%20Reference)))

(event EventTick
  (params (DeltaSeconds :type Float%20%28single-precision%29))
  (Transformation|SetActorLocation (+ (Variables|Default|GetStartlocation) (Math|Vector|MakeVector 0.0 0.0 (* (Math|Trig|Sin(Radians) (* (Variables|Default|GetSpeed) (Utilities|Time|GetGameTimeinSeconds))) (Variables|Default|GetHeight)))) false false)
  (Transformation|AddLocalRotation (Variables|Default|GetRotation) (Math|Rotator|MakeRotator 0.0 0.0 (* DeltaSeconds (Variables|Default|GetRspeed))) false false))

(fn ConstructionScript)